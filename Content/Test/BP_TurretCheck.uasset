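; Test turret actor that detects the third-person character and fires bullets from two spawn points.
; Pawn sensing drives interpolated look-at rotation, with yaw on the actor and clamped pitch plus yaw on the Tower component.
; Each sighting also restarts a short retriggerable delay before spawning the bullet pair.
; Overlapping the Collision component snaps the actor's pitch and yaw to a look-at rotation without interpolation.
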(event OnSeePawn(PawnSensing)
  (params (Pawn :type Pawn%20Object%20Reference))
  (bind _returnvalue (Transformation|GetActorLocation))
  (bind _returnvalue_2 (Transformation|GetActorLocation))
  (bind _returnvalue_3 (Utilities|Time|GetWorldDeltaSeconds))
  (bind _returnvalue_4 (Transformation|GetActorRotation))
  (bind _returnvalue_5 (* 2e+01 5.0))
  (bind _returnvalue_6 (Math|Rotator|FindLookatRotation _returnvalue _returnvalue_2))
  (bind _returnvalue_7 (Math|Interpolation|RInterpTo _returnvalue_4 _returnvalue_6 _returnvalue_3 _returnvalue_5))
  (Utilities|Casting|CastToBP_ThirdPersonCharacter Pawn)
  (Utilities|FlowControl|Sequence
    (:then_0
      (Transformation|SetWorldRotation (Variables|Default|GetTower) (Math|Rotator|MakeRotator 0.0 (Math|Float|Clamp(Float) (.pitch _returnvalue_7) -2e+01 2e+01) (.yaw _returnvalue_7)) false false)
      (Transformation|SetActorRotation (Math|Rotator|MakeRotator 0.0 0.0 (.yaw _returnvalue_7))))
    (:then_1
      (Utilities|FlowControl|RetriggerableDelay 0.2)
      (Game|SpawnActorfromClass "/Game/Test/BP_Bullet.BP_Bullet_C" (Transformation|GetWorldTransform (Variables|Default|GetBulletSpawn)) "Undefined" 0 0)
      (Game|SpawnActorfromClass "/Game/Test/BP_Bullet.BP_Bullet_C" (Transformation|GetWorldTransform (Variables|Default|GetBulletSpawn1)) "Undefined" 0 0))))

(event OnComponentBeginOverlap(Collision)
  (params (OverlappedComponent :type Primitive%20Component%20Object%20Reference) (OtherActor :type Actor%20Object%20Reference) (OtherComp :type Primitive%20Component%20Object%20Reference) (OtherBodyIndex :type Integer) (bFromSweep :type Boolean) (SweepResult :type Hit%20Result%20Structure%20%28by%20ref%29))
  (bind _returnvalue (Transformation|GetActorLocation))
  (bind _returnvalue_2 (Transformation|GetActorLocation))
  (bind _returnvalue_3 (Math|Rotator|FindLookatRotation _returnvalue _returnvalue_2))
  (Utilities|Casting|CastToBP_ThirdPersonCharacter OtherActor)
  (Transformation|SetActorRotation (Math|Rotator|MakeRotator 0.0 (.pitch _returnvalue_3) (.yaw _returnvalue_3))))

(fn ConstructionScript)