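; Attack component for BP_Undead enemies that plays zombie melee montages on the owner's mesh, with the scaffolding for a three-hit combo.
; Undeadattack starts or buffers an attack, and UndeadComboattack consumes the buffer or resets via StopCombo.
; The AttackIndex switch only calls Attack1; Attack2 and Attack3 have delayed, DoOnce-gated montages but no caller here.
; AttackTrace starts a looping timer whose trace event is still empty.
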(event Custom|Undead%20attack
  (if (Variables|Default|GetAttacking?)
    (Variables|Default|SetSave%20Attack? true)
    (else
      (Variables|Default|SetAttacking? true)
      (switch int (Variables|Default|GetAttack%20index)
        (:0
          (CallFunction|Attack1))))))

(event Custom|Undead%20Combo%20attack
  (if (Variables|Default|GetSave%20Attack?)
    (Variables|Default|SetSave%20Attack? false)
    (switch int (Variables|Default|GetAttack%20index)
      (:0
        (CallFunction|Attack1)))
    (else
      (CallFunction|StopCombo))))

(event Custom|Stop%20combo
  (Variables|Default|SetAttacking? false)
  (Variables|Default|SetAttack%20index 0))

(event Custom|Attack3
  (Utilities|FlowControl|DoOnce false :!label _label
    (:Completed
      (Utilities|FlowControl|Delay 0.2)
      (Animation|Montage|PlayMontage (Variables|Default|GetMesh) "/Game/Enemy/Undead/Animation/Attack/Zombie_Attack_13_Montage.Zombie_Attack_13_Montage"
        (:then
          (Variables|Default|SetAttack%20index 2)
          (goto _label Reset))))))

(event Custom|Attack1
  (Utilities|FlowControl|DoOnce false :!label _label
    (:Completed
      (Utilities|FlowControl|Delay 0.2)
      (Animation|Montage|PlayMontage (Variables|Default|GetMesh) "/Game/Enemy/Undead/Animation/Attack/Zombie_Attack_11_Montage.Zombie_Attack_11_Montage"
        (:then
          (Variables|Default|SetAttack%20index 0)
          (goto _label Reset))))))

(event Custom|Attack%20trace%20Loop)

(event Custom|Attack2
  (Utilities|FlowControl|DoOnce false :!label _label
    (:Completed
      (Utilities|FlowControl|Delay 0.2)
      (Animation|Montage|PlayMontage (Variables|Default|GetMesh) "/Game/Enemy/Undead/Animation/Attack/Zombie_Attack_12_Montage.Zombie_Attack_12_Montage"
        (:then
          (Variables|Default|SetAttack%20index 1)
          (goto _label Reset))))))

(event Custom|Attack%20Trace
  (Utilities|Time|SetTimerbyEvent (delegate Custom|Attack%20trace%20Loop) 0.1 true))

(event Input|EnhancedActionEvents|EnhancedInputActionIA_Attack
  (params (ActionValue :type Boolean) (ElapsedSeconds :type Float%20%28double-precision%29) (TriggeredSeconds :type Float%20%28double-precision%29) (InputAction :type Input%20Action%20Object%20Reference :default "/Game/ThirdPerson/Input/Actions/IA_Attack.IA_Attack")))

(event EventBeginPlay
  (bind _asbp_undead (Utilities|Casting|CastToBP_Undead (Components|GetOwner)))
  (Variables|Default|SetMesh (Variables|/Script/Engine.Character|GetMesh _asbp_undead)))

(event EventTick
  (params (DeltaSeconds :type Float%20%28single-precision%29)))