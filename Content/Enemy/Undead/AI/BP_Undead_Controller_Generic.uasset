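; Generic AI controller for undead enemies that starts the enemy behavior tree on BeginPlay.
; On each AI Perception update, it writes the first updated actor into the TargetTurret blackboard key, without checking sense type or whether sensing succeeded.
; A sight-filtered version that sets TargetTurret or clears a differently named Target key is disconnected, and its OnTargetPerceptionUpdated event is empty.
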(event OnPerceptionUpdated(AIPerception)
  (params (UpdatedActors :type Array%20of%20Actor%20Object%20References))
  (AI|Components|Blackboard|SetValueasObject (Variables|Default|GetBlackboard) (Utilities|Name|MakeLiteralName "TargetTurret") (Utilities|Array|Get(acopy) UpdatedActors)))

(event OnTargetPerceptionUpdated(AIPerception)
  (params (Actor :type Actor%20Object%20Reference) (Stimulus :type AI%20Stimulus%20Structure)))

(event EventBeginPlay
  (AI|RunBehaviorTree "/Game/Enemy/Undead/AI/EnemyBehaviorTree.EnemyBehaviorTree"))

(fn ConstructionScript)