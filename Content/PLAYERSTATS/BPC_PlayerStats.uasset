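; Player stats component that tracks current and maximum health and stamina for BP_ThirdPersonCharacter1.
; One tick after BeginPlay it caches the owning character and initializes its HUD bars and health text.
; Functions change each stat and refresh the HUD directly, with the decrease functions returning true on depletion.
; IncreaseHealth sets health to zero because its addition node is unconnected, while IncreaseStamina adds and clamps to the maximum.
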(event EventBeginPlay
  (Utilities|FlowControl|DelayUntilNextTick)
  (bind _asbp_third_person_character_1 (Utilities|Casting|CastToBP_ThirdPersonCharacter1 (Components|GetOwner)))
  (Variables|Default|SetPlayerCharacter%20BP _asbp_third_person_character_1)
  (Progress|SetPercent (Variables|/Game/PLAYERSTATS/UI/WB_MainHud.WB_MainHud_C|GetStaminaBar (Variables|/Game/ThirdPersonCPP/Blueprints/BP_ThirdPersonCharacter1.BP_ThirdPersonCharacter1_C|GetHudWidget (Variables|Default|GetPlayerCharacter%20BP))) (/ (Variables|Stamina|GetCurrent%20Stamina) (Variables|Stamina|GetMax%20Stamina)))
  (Progress|SetPercent (Variables|/Game/PLAYERSTATS/UI/WB_MainHud.WB_MainHud_C|GetHealthBar (Variables|/Game/ThirdPersonCPP/Blueprints/BP_ThirdPersonCharacter1.BP_ThirdPersonCharacter1_C|GetHudWidget (Variables|Default|GetPlayerCharacter%20BP))) (/ (Variables|Health|GetCurrent%20Health) (Variables|Health|GetMax%20Health)))
  (Rendering|Components|TextRender|SetText (Variables|/Game/PLAYERSTATS/UI/WB_MainHud.WB_MainHud_C|GetHealthText (Variables|/Game/ThirdPersonCPP/Blueprints/BP_ThirdPersonCharacter1.BP_ThirdPersonCharacter1_C|GetHudWidget (Variables|Default|GetPlayerCharacter%20BP))) (Utilities|Text|ToText(Float) (Variables|Health|GetCurrent%20Health) "HalfToEven")))

(fn DecreaseHealth
  (params (Damage :type Float%20%28double-precision%29))
  (bind _playercharacter_bp (Variables|Default|GetPlayerCharacter%20BP))
  (bind _hudwidget (Variables|/Game/ThirdPersonCPP/Blueprints/BP_ThirdPersonCharacter1.BP_ThirdPersonCharacter1_C|GetHudWidget _playercharacter_bp))
  (if (not (<= (Variables|Health|GetCurrent%20Health) 0.0))
    (bind _output_get (Variables|Health|SetCurrent%20Health (- (Variables|Health|GetCurrent%20Health) Damage)))
    (Progress|SetPercent (Variables|/Game/PLAYERSTATS/UI/WB_MainHud.WB_MainHud_C|GetHealthBar _hudwidget) (/ _output_get (Variables|Health|GetMax%20Health)))
    (Rendering|Components|TextRender|SetText (Variables|/Game/PLAYERSTATS/UI/WB_MainHud.WB_MainHud_C|GetHealthText _hudwidget) (Utilities|Text|ToText(Float) (Variables|Health|GetCurrent%20Health) "HalfToEven"))
    (if (<= (Variables|Health|GetCurrent%20Health) 0.0)
      _
      (else
        (return false))))
  (return true))

(fn IncreaseMaxHealth
  (params (Incremention :type Float%20%28double-precision%29))
  (bind _playercharacter_bp (Variables|Default|GetPlayerCharacter%20BP))
  (bind _hudwidget (Variables|/Game/ThirdPersonCPP/Blueprints/BP_ThirdPersonCharacter1.BP_ThirdPersonCharacter1_C|GetHudWidget _playercharacter_bp))
  (Variables|Health|SetMax%20Health (+ (Variables|Health|GetMax%20Health) Incremention))
  (Progress|SetPercent (Variables|/Game/PLAYERSTATS/UI/WB_MainHud.WB_MainHud_C|GetHealthBar _hudwidget) (/ (Variables|Health|GetCurrent%20Health) (Variables|Health|GetMax%20Health)))
  (Rendering|Components|TextRender|SetText (Variables|/Game/PLAYERSTATS/UI/WB_MainHud.WB_MainHud_C|GetHealthText _hudwidget) (Utilities|Text|ToText(Float) (Variables|Health|GetCurrent%20Health) "HalfToEven")))

(fn IncreaseMaxStamina
  (params (Added%20Stamina :type Float%20%28double-precision%29))
  (Variables|Stamina|SetMax%20Stamina (+ (Variables|Stamina|GetMax%20Stamina) Added%20Stamina))
  (Progress|SetPercent (Variables|/Game/PLAYERSTATS/UI/WB_MainHud.WB_MainHud_C|GetStaminaBar (Variables|/Game/ThirdPersonCPP/Blueprints/BP_ThirdPersonCharacter1.BP_ThirdPersonCharacter1_C|GetHudWidget (Variables|Default|GetPlayerCharacter%20BP))) (/ (Variables|Stamina|GetCurrent%20Stamina) (Variables|Stamina|GetMax%20Stamina))))

(fn DecreaseStamina
  (params (Stamina%20Depleted :type Float%20%28double-precision%29))
  (if (not (<= (Variables|Stamina|GetCurrent%20Stamina) 0.0))
    (Variables|Stamina|SetCurrent%20Stamina (- (Variables|Stamina|GetCurrent%20Stamina) Stamina%20Depleted))
    (Progress|SetPercent (Variables|/Game/PLAYERSTATS/UI/WB_MainHud.WB_MainHud_C|GetStaminaBar (Variables|/Game/ThirdPersonCPP/Blueprints/BP_ThirdPersonCharacter1.BP_ThirdPersonCharacter1_C|GetHudWidget (Variables|Default|GetPlayerCharacter%20BP))) (/ (Variables|Stamina|GetCurrent%20Stamina) (Variables|Stamina|GetMax%20Stamina)))
    (if (<= (Variables|Stamina|GetCurrent%20Stamina) 0.0)
      _
      (else
        (return false))))
  (return true))

(fn IncreaseHealth
  (params (Added%20Health :type Float%20%28double-precision%29))
  (bind _playercharacter_bp (Variables|Default|GetPlayerCharacter%20BP))
  (bind _hudwidget (Variables|/Game/ThirdPersonCPP/Blueprints/BP_ThirdPersonCharacter1.BP_ThirdPersonCharacter1_C|GetHudWidget _playercharacter_bp))
  (Variables|Health|SetCurrent%20Health 0.0)
  (if (> (Variables|Health|GetCurrent%20Health) (Variables|Health|GetMax%20Health))
    (Variables|Health|SetCurrent%20Health (Variables|Health|GetMax%20Health)))
  (Progress|SetPercent (Variables|/Game/PLAYERSTATS/UI/WB_MainHud.WB_MainHud_C|GetHealthBar _hudwidget) (/ (Variables|Health|GetCurrent%20Health) (Variables|Health|GetMax%20Health)))
  (Rendering|Components|TextRender|SetText (Variables|/Game/PLAYERSTATS/UI/WB_MainHud.WB_MainHud_C|GetHealthText _hudwidget) (Utilities|Text|ToText(Float) (Variables|Health|GetCurrent%20Health) "HalfToEven")))

(fn IncreaseStamina
  (params (Added%20Stamina :type Float%20%28double-precision%29))
  (Variables|Stamina|SetCurrent%20Stamina (+ (Variables|Stamina|GetCurrent%20Stamina) Added%20Stamina))
  (if (> (Variables|Stamina|GetCurrent%20Stamina) (Variables|Stamina|GetMax%20Stamina))
    (Variables|Stamina|SetCurrent%20Stamina (Variables|Stamina|GetMax%20Stamina)))
  (Progress|SetPercent (Variables|/Game/PLAYERSTATS/UI/WB_MainHud.WB_MainHud_C|GetStaminaBar (Variables|/Game/ThirdPersonCPP/Blueprints/BP_ThirdPersonCharacter1.BP_ThirdPersonCharacter1_C|GetHudWidget (Variables|Default|GetPlayerCharacter%20BP))) (/ (Variables|Stamina|GetCurrent%20Stamina) (Variables|Stamina|GetMax%20Stamina))))